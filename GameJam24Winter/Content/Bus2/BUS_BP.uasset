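; BUS_BP is a bus actor that changes its seating setup when play begins in Level4.
; On BeginPlay it checks the level name, swaps the bus mesh to the chairless variant and makes its four separate chair components visible.
; The mesh swap targets the bus found through GetActorOfClass rather than self, while the chair changes apply to its own components.
; Overlap, Tick and the construction script are empty.
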(event `self.ReceiveBeginPlay`
  (bind _returnvalue (`GameplayStatics.GetCurrentLevelName` true))
  (if (`KismetStringLibrary.EqualEqual_StrStr` _returnvalue "Level4")
    (bind _returnvalue_2 (`GameplayStatics.GetActorOfClass` "BUS_BP_C"))
    (`StaticMeshComponent.SetStaticMesh` (`/Game/Bus2/BUS_BP.BusMesh` _returnvalue_2) "/Game/Bus2/Bus_NoChair.Bus_NoChair")
    (`SceneComponent.SetVisibility` (`self.BusChair`) true false)
    (`SceneComponent.SetVisibility` (`self.BusChair1`) true false)
    (`SceneComponent.SetVisibility` (`self.BusChair2`) true false)
    (`SceneComponent.SetVisibility` (`self.BusChair3`) true false)))

(fn `UserConstructionScript`)